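; BP_BombBallMode handles respawning of the player's BP_BombBallCharacter in the Bomb Ball game.
; On BeginPlay it binds to the destroyed event of player 0's character.
; When that character is destroyed, it waits a zero-length delay, spawns a replacement at SpawnTransform and has player controller 0 possess it.
; It then calls Respawn to bind the new character, repeating the cycle, and prints a debug message.
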(event Custom|On_Destroy_Event
  (Utilities|FlowControl|Delay 0.0)
  (bind _returnvalue (Game|SpawnActorfromClass "/Game/BombBallBlueprints/BP_BombBallCharacter.BP_BombBallCharacter_C" (Variables|Default|GetSpawn_Transform) "Undefined" 0 0))
  (Pawn|Possess (Game|GetPlayerController 0) _returnvalue)
  (CallFunction|Respawn)
  (Development|PrintText "respawn"))

(event Custom|Respawn
  (bind _asbp_bomb_ball_character (Utilities|Casting|CastToBP_BombBallCharacter (Game|GetPlayerCharacter 0)))
  (Game|BindEventtoOnDestroyed _asbp_bomb_ball_character (delegate Custom|On_Destroy_Event)))

(event EventBeginPlay
  (bind _asbp_bomb_ball_character (Utilities|Casting|CastToBP_BombBallCharacter (Game|GetPlayerCharacter 0)))
  (Game|BindEventtoOnDestroyed _asbp_bomb_ball_character (delegate Custom|On_Destroy_Event)))

(event EventTick
  (params (DeltaSeconds :type Float%20%28single-precision%29)))

(fn ConstructionScript)